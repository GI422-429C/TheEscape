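; BP_NPC is a talkable NPC that shows its lines from a Dialogue array one at a time.
; Overlap begin and end toggle its Widget component, and BeginPlay adds a quest widget to the viewport.
; Each Talk call advances Talkindex, updates a lazily created WB_DialogueNPC, removes the quest widget and hides the component.
; Once the lines run out, Talk removes the dialogue UI without resetting the index.
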(event `self.ReceiveBeginPlay`
  (bind _returnvalue (`|CreateWidget` "/Game/Quest/WB_Quest.WB_Quest_C"))
  (`UserWidget.AddToViewport` _returnvalue 0))

(event `/Game/npc/men/BPI_Dialogue.Talk`
  (`/Engine/EditorBlueprintResources/StandardMacros.IncrementInt` (`self.talkindex`)
    (:`  `
      (if (< (`self.talkindex`) (`KismetArrayLibrary.Array_Length` (`self.dialogue`)))
        (`self.UI`
          (:`then`
            _)
          (:`else`
            (bind _returnvalue (`|CreateWidget` "/Game/npc/men/WB_DialogueNPC.WB_DialogueNPC_C" (`GameplayStatics.GetPlayerController` 0)))
            (bind _output_get (set `self.UI` _returnvalue))
            (`UserWidget.AddToViewport` _output_get 0)))
        (`TextBlock.SetText` (`/Game/npc/men/WB_DialogueNPC.TalkNPC` (`self.UI`)) (`KismetTextLibrary.Conv_StringToText` (`|GetArrayItem` (`self.dialogue`) (`self.talkindex`))))
        (`Widget.RemoveFromParent` (stale `self.ReceiveBeginPlay` _returnvalue))
        (`SceneComponent.SetVisibility` (`self.Widget`) false false)
        (else
          (`Widget.RemoveFromParent` (`self.UI`)))))))

(event `self.ReceiveActorBeginOverlap`
  (params (OtherActor :type "Actor Object Reference"))
  (`SceneComponent.SetVisibility` (`self.Widget`) true false))

(event `self.ReceiveActorEndOverlap`
  (params (OtherActor :type "Actor Object Reference"))
  (`SceneComponent.SetVisibility` (`self.Widget`) false false))

(fn `UserConstructionScript`)