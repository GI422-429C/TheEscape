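; BP_PuzzleGate is a gate that opens only after enough items have been collected.
; Collectitem increments the count, and Opendoorcheck compares it to the required maximum, then either opens the gate once or briefly shows a BP_HavetoKey widget, with a lock sound.
; A timeline swings the door's yaw open.
; Actor overlap toggles the visibility of a prompt widget, commented as "E to open".
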(event `Open Door`
  (bind (_direction _door_rotation) (`Timeline|Open Door Anim`)
    (:`Update`
      (`SceneComponent.K2_SetRelativeRotation` (`self.Door`) (`KismetMathLibrary.MakeRotator` 0.0 0.0 (`KismetMathLibrary.Lerp` 0.0 270.0 _door_rotation)) false false))))

(event `Collect item`
  (`/Engine/EditorBlueprintResources/StandardMacros.IncrementInt` (`self.currentItemsCollect`)))

(event `Open door check`
  (if (>= (`self.currentItemsCollect`) (`self.MaxItemsCollecatble`))
    (`/Engine/EditorBlueprintResources/StandardMacros.DoOnce` false
      (:`Completed`
        (`GameplayStatics.PlaySound2D` "/Game/sound/door-lock-43124.door-lock-43124" 1.0 1.0 0.0 null null)
        (`self.Open Door`)))
    (else
      (`GameplayStatics.PlaySound2D` "/Game/sound/door-lock-43124.door-lock-43124" 1.0 1.0 0.0 null null)
      (bind _returnvalue (`|CreateWidget` "/Game/door/BP_HavetoKey.BP_HavetoKey_C"))
      (`UserWidget.AddToViewport` _returnvalue 0)
      (`KismetSystemLibrary.Delay` 2.0)
      (`Widget.RemoveFromParent` _returnvalue))))

(event `self.ReceiveActorBeginOverlap`
  (params (OtherActor :type "Actor Object Reference"))
  ;[1 1 1] E to open
  (`SceneComponent.SetVisibility` (`self.Widget`) true false))

(event `self.ReceiveActorEndOverlap`
  (params (OtherActor :type "Actor Object Reference"))
  ;[1 1 1] E to open
  (`SceneComponent.SetVisibility` (`self.Widget`) false false))

(fn `UserConstructionScript`)